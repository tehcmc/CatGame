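; Base pickup Blueprint that manages a mesh's custom-depth highlight and its drop physics.
; Activating or deactivating the OutlineComponent toggles custom depth rendering on the mesh, which starts disabled on BeginPlay.
; Being picked up also clears custom depth, and being dropped turns on physics simulation for the mesh.
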(event `self.ReceiveBeginPlay`
  (`PrimitiveComponent.SetRenderCustomDepth` (`self.MeshComponent`) false))

(event `self.OnPickup`
  (`PrimitiveComponent.SetRenderCustomDepth` (`self.MeshComponent`) false))

(event `self.OnDropped`
  (`PrimitiveComponent.SetSimulatePhysics` (`self.MeshComponent`) true))

(event `self.OutlineComponent.OnComponentActivated`
  (params (Component :type "ActorComponent Object Reference") (bReset :type Boolean))
  (`PrimitiveComponent.SetRenderCustomDepth` (`self.MeshComponent`) true))

(event `self.OutlineComponent.OnComponentDeactivated`
  (params (Component :type "ActorComponent Object Reference"))
  (`PrimitiveComponent.SetRenderCustomDepth` (`self.MeshComponent`) false))

(fn `UserConstructionScript`)