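; CandleWick is a candle wick actor that starts lit or is ignited by overlapping an actor tagged "Flame".
; On BeginPlay, PreLit turns on the flame effect, point light and cube material swap, while an unlit wick clears its tags.
; Ignition adds the "Flame" tag and applies the same visuals, with the tag also serving as the lit state.
; A getter exposes BurntOut, which nothing here sets.
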(event `self.ReceiveBeginPlay`
  (if (`self.PreLit`)
    (`ActorComponent.SetActive` (`self.Flames`) true false)
    (`SceneComponent.SetVisibility` (`self.PointLight`) true false)
    (`PrimitiveComponent.SetMaterial` (`self.Cube`) 0 "/Engine/EngineMeshes/BackgroundMaterial.BackgroundMaterial")
    (else
      (`KismetArrayLibrary.Array_Clear` (`self.Tags`)))))

(event `self.ReceiveActorBeginOverlap`
  (params (OtherActor :type "Actor Object Reference"))
  (if (not (`self.PreLit`))
    ;[1 1 1] Check if interaction has flame tag and light match head if it does
    (if (`self.ActorHasTag` OtherActor "Flame")
      (if (`self.ActorHasTag` self "Flame")
        (`KismetSystemLibrary.PrintString` "Already on fire")
        (else
          (`KismetArrayLibrary.Array_Add` (`self.Tags`) "Flame")
          (`ActorComponent.SetActive` (`self.Flames`) true false)
          (`SceneComponent.SetVisibility` (`self.PointLight`) true false)
          (`PrimitiveComponent.SetMaterial` (`self.Cube`) 0 "/Engine/EngineMeshes/BackgroundMaterial.BackgroundMaterial"))))))

(fn `Get Burnt out`
  (returns (Burnt :type Boolean))
  (return (`self.BurntOut`)))

(fn `UserConstructionScript`)