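; A test actor for a breakable Chaos object that falls apart and removes itself from the world.
; OnInteract prints a debug message and turns on physics simulation for the Smashy component.
; Smashy's first Chaos break event prints a smash message, sets HasBroken, switches off break notifications and destroys the actor after a short delay.
; Any further break event only switches notifications off again.
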(event `self.OnInteract`
  (`KismetSystemLibrary.PrintString` "Hello")
  (`PrimitiveComponent.SetSimulatePhysics` (`self.Smashy`) true))

(event `self.Smashy.OnChaosBreakEvent`
  (params (BreakEvent :type "ChaosBreakEvent Structure (by ref)"))
  (bind _smashy (`self.Smashy`))
  (if (`self.HasBroken`)
    (`GeometryCollectionComponent.SetNotifyBreaks` _smashy false)
    (else
      (`KismetSystemLibrary.PrintString` "SMASH!!!!!!!!")
      (set `self.HasBroken` true)
      (`GeometryCollectionComponent.SetNotifyBreaks` _smashy false)
      (`KismetSystemLibrary.Delay` 5.0)
      (`self.K2_DestroyActor`))))

(fn `UserConstructionScript`)