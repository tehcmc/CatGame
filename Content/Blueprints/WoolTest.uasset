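; Test wool actor that rolls along a referenced track's spline while a CatBase actor overlaps it.
; Overlap begin plays a timeline with its rate set from Duration, and overlap end stops it in place, so the next overlap resumes.
; The timeline alpha maps to distance along the spline, setting world location and rotation while scaling the wool with progress.
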(event `self.ReceiveBeginPlay`)

(event `self.ReceiveActorBeginOverlap`
  (params (OtherActor :type "Actor Object Reference"))
  (cast `CatBase` OtherActor)
  (`self.Move Wool`))

(event `self.ReceiveActorEndOverlap`
  (params (OtherActor :type "Actor Object Reference"))
  (cast `CatBase` OtherActor)
  (`self.StopWool`))

(event `Move Wool`
  (bind _returnvalue (`KismetMathLibrary.Lerp` 0.0 (`SplineComponent.GetSplineLength` (`/Game/Blueprints/WoolPath.Spline` (`self.TrackRef`))) (`self.Alpha`)))
  (`TimelineComponent.SetPlayRate` (`self.Timeline`) (/ 1.0 (`self.Duration`)))
  (bind (_direction _alpha) (`Timeline|Timeline` :!label _label)
    (:`Update`
      (bind _output_get (set `self.Alpha` _alpha))
      (`self.SetActorScale3D` (`KismetMathLibrary.Conv_DoubleToVector` (* (+ _output_get 1.0) 1.2)))
      (`self.K2_SetActorLocationAndRotation` (`SplineComponent.GetLocationAtDistanceAlongSpline` (`/Game/Blueprints/WoolPath.Spline` (`self.TrackRef`)) _returnvalue "World") (`SplineComponent.GetRotationAtDistanceAlongSpline` (`/Game/Blueprints/WoolPath.Spline` (`self.TrackRef`)) _returnvalue "World")))))

(event `StopWool`
  (goto _label :!via `Stop`))

(fn `UserConstructionScript`)