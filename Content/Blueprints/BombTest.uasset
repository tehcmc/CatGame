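; BombTest is a test bomb actor that ignites when it overlaps an actor tagged "Flame".
; Ignition turns on Sparks, then a fixed delay leads to a debug print, a RadialForce impulse sized from the BombRadius sphere, and the actor's destruction.
; The overlap is gated on the Lit flag, but this graph never sets it.
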(event `self.ReceiveBeginPlay`)

(event `self.ReceiveActorBeginOverlap`
  (params (OtherActor :type "Actor Object Reference"))
  (bind _radialforce (`self.RadialForce`))
  (if (`self.Lit`)
    _
    (elif (`self.ActorHasTag` OtherActor "Flame")
      (`ActorComponent.SetActive` (`self.Sparks`) true false)
      (`KismetSystemLibrary.Delay` 5.0)
      (`KismetSystemLibrary.PrintString` "boom" true true (struct :`R` 1.0 :`B` 0.019485 :`A` 1.0))
      (set `RadialForceComponent.Radius` (`SphereComponent.SphereRadius` (`self.BombRadius`)) _radialforce)
      (`RadialForceComponent.FireImpulse` _radialforce)
      (`self.K2_DestroyActor`))))

(fn `UserConstructionScript`)