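; Flammable paper actor that catches fire when it overlaps an actor tagged Flame.
; It clears its tags on BeginPlay, then on ignition adds the Flame tag to itself, which marks it as a fire source, and activates flame effects and sound.
; The actor destroys itself after a fixed burn delay.
; An IsBurning check guards ignition, but this graph never sets that variable.
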(event `self.ReceiveBeginPlay`
  (`KismetArrayLibrary.Array_Clear` (`self.Tags`)))

(event `self.ReceiveActorBeginOverlap`
  (params (OtherActor :type "Actor Object Reference"))
  (if (`self.ActorHasTag` OtherActor "Flame")
    (if (not (`self.IsBurning`))
      (`KismetArrayLibrary.Array_Add` (`self.Tags`) "Flame")
      (`ActorComponent.Activate` (`self.Flames`) false)
      (`AudioComponent.Play` (`self.Fire Sound`) 0.0)
      (`KismetSystemLibrary.Delay` 20.0)
      (`self.K2_DestroyActor`))))

(fn `UserConstructionScript`)