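; MatchHead is an actor for a match tip that lights when it overlaps an actor tagged Flame.
; Once lit it takes the Flame tag itself, so it can ignite others, and turns on its flame effect and point light.
; After BurnTime it clears its tags, switches the effects off, swaps the cube material and sets BurntOut, which blocks relighting and is exposed through GetBurntOut.
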(event `self.ReceiveBeginPlay`
  (`KismetArrayLibrary.Array_Clear` (`self.Tags`)))

(event `self.ReceiveActorBeginOverlap`
  (params (OtherActor :type "Actor Object Reference"))
  (bind _tags (`self.Tags`))
  (bind _pointlight (`self.PointLight`))
  (bind _flames (`self.Flames`))
  ;[1 1 1] Check if interaction has flame tag and light match head if it does
  (if (`self.ActorHasTag` OtherActor "Flame")
    (if (`self.ActorHasTag` self "Flame")
      (`KismetSystemLibrary.PrintString` "Already on fire")
      (elif (`self.BurntOut`)
        (`KismetSystemLibrary.PrintString` "Burnt out" true true (struct :`R` 1.0 :`G` 0.041795 :`A` 1.0))
        (else
          (`KismetArrayLibrary.Array_Add` _tags "Flame")
          (`ActorComponent.SetActive` _flames true false)
          (`SceneComponent.SetVisibility` _pointlight true false)
          (`KismetSystemLibrary.Delay` (`self.BurnTime`))
          (`KismetArrayLibrary.Array_Clear` _tags)
          (`ActorComponent.SetActive` _flames false false)
          (`SceneComponent.SetVisibility` _pointlight false false)
          (`PrimitiveComponent.SetMaterial` (`self.Cube`) 0 "/DatasmithContent/Materials/C4DReference.C4DReference")
          (set `self.BurntOut` true))))))

(fn `Get Burnt out`
  (returns (Burnt :type Boolean))
  (return (`self.BurntOut`)))

(fn `UserConstructionScript`)