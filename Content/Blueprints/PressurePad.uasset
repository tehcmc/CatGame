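; A weighted pressure pad that sinks its button under a heavy enough actor and triggers an Activator.
; An actor overlapping the button collider whose primitive component mass meets the threshold plays a Timeline that moves the button.
; When the Timeline finishes, an overlap between SparkBox and TriggerBox calls ButtonCompleted, which activates the Activator.
; Any actor ending overlap reverses the Timeline, without collider or mass checks.
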(event `self.ReceiveActorBeginOverlap`
  (params (OtherActor :type "Actor Object Reference"))
  (if (`PrimitiveComponent.IsOverlappingActor` (`self.ButtonCollider`) OtherActor)
    (if (>= (`PrimitiveComponent.GetMass` (`self.GetComponentByClass` OtherActor "/Script/Engine.PrimitiveComponent")) (`self.MassThreshold`))
      (bind (_direction _newtrack_0) (`Timeline|Timeline` :!label _label)
        (:`Update`
          (`SceneComponent.K2_SetRelativeLocation` (`self.Button`) _newtrack_0 false false))
        (:`Finished`
          (if (`PrimitiveComponent.IsOverlappingComponent` (`self.SparkBox`) (`self.TriggerBox`))
            (`self.ButtonCompleted`)))))))

(event `self.ReceiveActorEndOverlap`
  (params (OtherActor :type "Actor Object Reference"))
  (goto _label :!via `Reverse`))

(event `ButtonCompleted`
  (`ActorComponent.Activate` (`self.Activator`) false))

(fn `UserConstructionScript`)