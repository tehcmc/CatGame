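; Test sliding door that moves its mesh along relative Z when a child-actor pressure pad is activated.
; On BeginPlay it casts the Button child to PressurePad and binds OpenDoor to the pad Activator's activation event.
; A Timeline drives the motion; when it finishes with IsFinished false, a delay precedes deactivating the Activator and reversing the Timeline.
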(event `self.ReceiveBeginPlay`
  (bind _aspressure_pad (cast `/Game/Blueprints/PressurePad` (`ChildActorComponent.ChildActor` (`self.Button`))))
  (set `self.PadRef` _aspressure_pad)
  (add `ActorComponent.OnComponentActivated` (`/Game/Blueprints/PressurePad.Activator` (`self.PadRef`)) (delegate `OpenDoor`)))

(event `OpenDoor`
  (params (Component :type "ActorComponent Object Reference") (bReset :type Boolean))
  (bind _staticmesh (`self.StaticMesh`))
  (bind (_direction _newtrack_0) (`Timeline|Timeline` :!label _label)
    (:`Update`
      (`SceneComponent.K2_SetRelativeLocation` _staticmesh (`KismetMathLibrary.MakeVector` (.x (`SceneComponent.RelativeLocation` _staticmesh)) (.y (`SceneComponent.RelativeLocation` _staticmesh)) (`.Z` (`KismetMathLibrary.BreakVector3f` _newtrack_0))) false false))
    (:`Finished`
      (if (not (`self.IsFinished`))
        (`KismetSystemLibrary.Delay` 10.0)
        (`ActorComponent.Deactivate` (`/Game/Blueprints/PressurePad.Activator` (`self.PadRef`)))
        (goto _label :!via `Reverse`)))))

(fn `UserConstructionScript`)