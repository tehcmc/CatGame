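; TestItem2 is a breakable item that the player's cat can hit to earn points, apparently a test asset.
; On its first successful OnHit, it casts the player character to CatBase and pushes the Breakable component along the cat's forward vector, scaled by PushForce, as an acceleration change.
; It then adds ScoreVal to the cat's score and sets HasScored, so later hits neither push nor score.
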(event `self.OnHit`
  (if (not (`self.HasScored`))
    (bind _ascat_base (cast `CatBase` (`GameplayStatics.GetPlayerCharacter` 0)))
    (`KismetSystemLibrary.PrintString` "Cast")
    (`PrimitiveComponent.AddForce` (`self.Breakable`) (* (`self.GetActorForwardVector` _ascat_base) (`KismetMathLibrary.Conv_DoubleToVector` (`self.Push force`))) "None" true)
    (`CatBase.SetScore` _ascat_base (+ (`CatBase.GetScore` _ascat_base) (`self.Score val`)))
    (set `self.HasScored` true)))

(fn `UserConstructionScript`)