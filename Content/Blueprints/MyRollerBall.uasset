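; MyRollerBall is a roller ball Blueprint that the player can exit to take control of a CatBase character.
; Overlapping a cat inside EntrySphere stores it as CatRef, while both mouse axes feed one node applying the same value to SpringArm pitch and yaw.
; Exit hides the ball's Cat component, teleports the unpossessed CatRef there, starts a view blend, possesses it and unhides it.
; Logic for hiding the cat on entry is unconnected.
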(event `InputAxisKey|MouseX`
  (params (AxisValue :type "Float (single-precision)"))
  (`SceneComponent.K2_AddRelativeRotation` (`self.SpringArm`) (`KismetMathLibrary.MakeRotator` 0.0 (stale `InputAxisKey|MouseY` AxisValue) AxisValue) false false :!label _label))

(event `InputAxisKey|MouseY`
  (params (AxisValue :type "Float (single-precision)"))
  (goto _label))

(event `self.ReceiveActorBeginOverlap`
  (params (OtherActor :type "Actor Object Reference"))
  (bind _ascat_base (cast `CatBase` OtherActor))
  (if (`PrimitiveComponent.IsOverlappingActor` (`self.EntrySphere`) _ascat_base)
    (set `self.CatRef` _ascat_base)))

(event `self.ExitPressed`
  (bind _catref (`self.CatRef`))
  (bind _cat (`self.Cat`))
  (bind _catref_2 (`self.CatRef`))
  (`/Engine/EditorBlueprintResources/StandardMacros.IsValid` _catref
    (:`Is Valid`
      (if (not (`self.IsPlayerControlled` _catref))
        (`SceneComponent.SetVisibility` _cat false false)
        (`self.K2_SetActorLocation` _catref_2 (`SceneComponent.K2_GetComponentLocation` _cat) false true)
        (`PlayerController.SetViewTargetWithBlend` (`GameplayStatics.GetPlayerController` 0) _catref_2 1.0 "VTBlend_Linear" 0.0 false)
        (`Controller.Possess` (`GameplayStatics.GetPlayerController` 0) _catref_2)
        (`self.SetActorHiddenInGame` _catref_2 false)))))

(fn `UserConstructionScript`)