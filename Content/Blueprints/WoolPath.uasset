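; WoolPath is an actor that uses a spline to lay out yarn test points along a path.
; On BeginPlay it loops over every spline point, prints the index for debugging and spawns a YarnPointTest at that point's world location.
; The construction script is empty, and an unconnected node for removing the first spline point never runs.
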(event `self.ReceiveBeginPlay`
  (for _index (range (`SplineComponent.GetNumberOfSplinePoints` (`self.Spline`)))
    (`KismetSystemLibrary.PrintString` (`KismetStringLibrary.Conv_IntToString` _index) true true (struct :`R` 1.0 :`G` 0.076571 :`A` 1.0))
    (`|SpawnActorFromClass` "/Game/Blueprints/YarnPointTest.YarnPointTest_C" (`KismetMathLibrary.Conv_VectorToTransform` (`SplineComponent.GetLocationAtSplinePoint` (`self.Spline`) _index "World")) "Undefined" "OverrideRootScale" null null)))

(fn `UserConstructionScript`)