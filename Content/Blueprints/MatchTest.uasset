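; A carryable match actor that burns out, falls apart under physics and then destroys itself.
; Its outline component toggles custom depth on the mesh, pickup clears that highlight, and dropping enables physics.
; Each tick polls the MatchHead child actor; once burnt out, it calls detach on the cat reference, enables physics on mesh and head, and destroys the actor after a delay.
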(event `self.ReceiveBeginPlay`
  (`PrimitiveComponent.SetRenderCustomDepth` (`self.MeshComponent`) false))

(event `self.OnPickup`
  (`PrimitiveComponent.SetRenderCustomDepth` (`self.MeshComponent`) false))

(event `self.OutlineComponent.OnComponentActivated`
  (params (Component :type "ActorComponent Object Reference") (bReset :type Boolean))
  (`PrimitiveComponent.SetRenderCustomDepth` (`self.MeshComponent`) true))

(event `self.OutlineComponent.OnComponentDeactivated`
  (params (Component :type "ActorComponent Object Reference"))
  (`PrimitiveComponent.SetRenderCustomDepth` (`self.MeshComponent`) false))

(event `self.ReceiveTick`
  (params (DeltaSeconds :type "Float (single-precision)"))
  (`self.BurnOut`)
  (if (`self.DestroyBegun`)
    (`KismetSystemLibrary.Delay` 5.0)
    (`self.K2_DestroyActor`)))

(event `self.OnDropped`
  (`PrimitiveComponent.SetSimulatePhysics` (`self.MeshComponent`) true))

(fn `BurnOut`
  (bind _returnvalue (`self.GetCatReference`))
  (if (not (`self.DestroyBegun`))
    (bind _asmatch_head (cast `/Game/Blueprints/MatchHead` (`ChildActorComponent.ChildActor` (`self.Head`))))
    (bind _burnt (`/Game/Blueprints/MatchHead.Get Burnt out` _asmatch_head))
    (if _burnt
      (set `self.DestroyBegun` true)
      (`/Engine/EditorBlueprintResources/StandardMacros.IsValid` _returnvalue
        (:`Is Valid`
          (`self.K2_DetachFromActor` _returnvalue "KeepRelative" "KeepRelative" "KeepRelative"))
        (:`Is Not Valid`
          _))
      (`PrimitiveComponent.SetSimulatePhysics` (`self.MeshComponent`) true)
      (`PrimitiveComponent.SetSimulatePhysics` (`/Game/Blueprints/MatchHead.Cube` _asmatch_head) true))))

(fn `UserConstructionScript`)